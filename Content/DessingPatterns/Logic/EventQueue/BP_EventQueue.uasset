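; BP_EventQueue is a demo of the Event Queue design pattern that drives timed image visibility changes in a UI widget.
; AddCommandToArray constructs a BP_ImageVisibility_CMD, appends it to CommandAR and fires CommandAdded.
; CommandAdded waits on a Delay, calls ChangeVisibilityImage on the player character's EQWidget, then re-calls itself while the array is non-empty.
; The graph itself never executes or removes the stored commands.
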(event Custom|CommandAdded
  (Utilities|FlowControl|Delay 2.0)
  (Default|ChangeVisibilityImage (Variables|Default|GetEQUIRef))
  (if (== (Utilities|Array|Length (Variables|Default|GetCommandAR)) 0)
    (Development|PrintString "No more actions")
    (else
      (CallFunction|CommandAdded))))

(event EventBeginPlay
  (Variables|Default|SetEQUIRef (Variables|/Game/TopDown/Blueprints/BP_TopDownCharacter.BP_TopDownCharacter_C|GetEQWidget (.AsBP%20Top%20Down%20Character (Utilities|Casting|CastToBP_TopDownCharacter (Game|GetPlayerCharacter 0))))))

(fn ConstructionScript)

(fn AddCommandtoArray
  (bind _returnvalue (Game|ConstructObjectfromClass "/Game/DessingPatterns/Logic/Command/BP_ImageVisibility_CMD.BP_ImageVisibility_CMD_C"))
  (Utilities|Array|Add (Variables|Default|GetCommandAR) _returnvalue)
  (CallFunction|CommandAdded))