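; BP_Flyweight is a demo of the Flyweight pattern that shares data table meshes across groups of placed Blueprints.
; On BeginPlay it reads the DTFWRow1 row and assigns its Mesh to every BPToAssignA element through AssignStaticMesh.
; The DTFWRow2 lookup sits inside that loop, so the assignment of its Mesh to all BPToAssignB elements repeats for each A element.
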(event EventBeginPlay
  (bind _dt_fwrow1 (Variables|Default|GetDT_FWRow1))
  (bind _dt_fwrow2 (Variables|Default|GetDT_FWRow2))
  (bind _returnvalue (Utilities|GetDataTableRow (.datatable _dt_fwrow1) (.rowname _dt_fwrow1))
    (:then
      (for _array_element (Variables|Default|GetBP_ToAssignA)
        (Default|AssignStaticMesh _array_element (Utilities|Struct|BreakS_Flyweight _returnvalue))
        (bind _returnvalue_2 (Utilities|GetDataTableRow (.datatable _dt_fwrow2) (.rowname _dt_fwrow2))
          (:then
            (for _array_element_2 (Variables|Default|GetBP_ToAssignB)
              (Default|AssignStaticMesh _array_element_2 (Utilities|Struct|BreakS_Flyweight _returnvalue_2)))))))))

(fn ConstructionScript)